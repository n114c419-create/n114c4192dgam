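; BP_PlayerCharactor01 is the player character, with side-to-side movement along world X and jumping.
; On BeginPlay it adds the IMC_Player01 Enhanced Input mapping context to player controller 0.
; Move input, gated by Canmove, drives AddMovementInput and sets IsFacingRight, which flips PlaySprite by rotating it 180 degrees.
; Blocked movement prints a debug string, while jump press and release call Jump and StopJumping regardless of that gate.
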(event Input|EnhancedActionEvents|EnhancedInputActionIA_Move01
  (params (ActionValue :type Vector%202D%20Structure) (ElapsedSeconds :type Float%20%28double-precision%29) (TriggeredSeconds :type Float%20%28double-precision%29) (InputAction :type Input%20Action%20Object%20Reference :default "/Game/myproject/input/IA_Move01.IA_Move01"))
  (bind _x (Math|Vector2D|BreakVector2D ActionValue))
  (bind _playsprite (Variables|Default|GetPlaySprite))
  (if (Variables|Default|Getcanmove)
    (if (> _x 0.0)
      (Variables|Default|SetIsFacingRight true)
      (else
        (Variables|Default|SetIsFacingRight false)))
    (Pawn|Input|AddMovementInput "0.500000,0.000000,0.000000" _x false)
    (if (Variables|Default|GetIsFacingRight)
      (Transformation|SetRelativeRotation _playsprite "0, 0, 0" false false)
      (else
        (Transformation|SetRelativeRotation _playsprite "0.000000,180.000000,0.000000" false false)))
    (else
      (Development|PrintString "movelocked"))))

(event Input|EnhancedActionEvents|EnhancedInputActionIA_Jump01
  (params (ActionValue :type Boolean) (ElapsedSeconds :type Float%20%28double-precision%29) (TriggeredSeconds :type Float%20%28double-precision%29) (InputAction :type Input%20Action%20Object%20Reference :default "/Game/myproject/input/IA_Jump01.IA_Jump01"))
  (:Started
    (Character|Jump))
  (:Completed
    (Character|StopJumping)))

(event EventBeginPlay
  (Input|AddMappingContext (PlayerController|LocalPlayerSubsystems|GetEnhancedInputLocalPlayerSubsystem (Game|GetPlayerController 0)) "/Game/myproject/input/IMC_Player01.IMC_Player01" 0 "(bIgnoreAllPressedKeysUntilRelease=True,bForceImmediately=False,bNotifyUserSettings=False)"))

(event Collision|EventActorBeginOverlap
  (params (OtherActor :type Actor%20Object%20Reference)))

(event EventTick
  (params (DeltaSeconds :type Float%20%28single-precision%29)))

(fn ConstructionScript)