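; Parallax backdrop actor that scrolls two background layers, SPFar and SPMid, along X as the player moves.
; BeginPlay records the player character's starting X, and Tick calls Updateparallax every frame.
; That function scales the player's X displacement by a separate factor per layer and teleports each to that relative location, with fixed depth offsets in Y and a lowered mid layer.
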(event EventBeginPlay
  (Variables|Default|SetPlayerstartx (.X (Math|Vector|BreakVector (Transformation|GetActorLocation (Game|GetPlayerCharacter 0))))))

(event Collision|EventActorBeginOverlap
  (params (OtherActor :type Actor%20Object%20Reference)))

(event EventTick
  (params (DeltaSeconds :type Float%20%28single-precision%29))
  (CallFunction|Updateparallax))

(fn ConstructionScript)

(fn Updateparallax
  (Variables|Default|SetDeltax (- (.X (Math|Vector|BreakVector (Transformation|GetActorLocation (Game|GetPlayerCharacter 0)))) (Variables|Default|GetPlayerstartx)))
  (Utilities|FlowControl|Sequence
    (:then_0
      (Transformation|SetRelativeLocation (Variables|Default|GetSP_far) (Math|Vector|MakeVector (+ (Variables|Default|Getxstart) (* (Variables|Default|GetDeltax) (Variables|Default|GetFarGB))) (+ (Variables|Default|Getystart) -2e+02) (Variables|Default|Getzstart)) false true))
    (:then_1
      (Transformation|SetRelativeLocation (Variables|Default|GetSP_mid) (Math|Vector|MakeVector (+ (Variables|Default|Getxstart) (* (Variables|Default|GetDeltax) (Variables|Default|Getmidbg))) (+ (Variables|Default|Getystart) -1e+02) (- (Variables|Default|Getzstart) 1e+02)) false true))))